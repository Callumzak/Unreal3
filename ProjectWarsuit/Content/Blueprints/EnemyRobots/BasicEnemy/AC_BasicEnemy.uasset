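; AI controller for the basic robot enemy that tracks the player through AI perception.
; On possess, it runs BT_BasicEnemy and stores the player character as the attack target in the Blackboard.
; Sensing a Player-tagged actor sets the line-of-sight and enemy keys and cancels the loss timer.
; Any other perception update starts a timeout that clears both keys, so the enemy keeps awareness briefly after losing sight.
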(event `self.ReceivePossess`
  (params (PossessedPawn :type "Pawn Object Reference"))
  ; Setting The Enemy Target
  (`self.RunBehaviorTree` "/Game/Blueprints/EnemyRobots/BasicEnemy/BT_BasicEnemy.BT_BasicEnemy")
  (`BlackboardComponent.SetValueAsObject` (`self.Blackboard`) (`self.Attack Target Key Name`) (`GameplayStatics.GetPlayerCharacter` 0)))

(event `self.AIPerception.OnTargetPerceptionUpdated`
  (params (Actor :type "Actor Object Reference") (Stimulus :type "AIStimulus Structure"))
  (bind _blackboard (`self.Blackboard`))
  ; Check for Player Visibility
  (if (and (`.bSuccessfullySensed` (break `AIStimulus` Stimulus)) (`self.ActorHasTag` Actor "Player"))
    (`KismetSystemLibrary.K2_ClearAndInvalidateTimerHandle` (`self.EnemyTimer`))
    ; Enemy Has Seen Player
    (`BlackboardComponent.SetValueAsBool` _blackboard (`self.HasLineOfSight`) true)
    (`BlackboardComponent.SetValueAsObject` _blackboard (`self.EnemyActor`) Actor)
    (else
      (bind _returnvalue (`KismetSystemLibrary.K2_SetTimerDelegate` (delegate `StartEnemyTimer`) (`self.LOStimeout`)))
      (set `self.EnemyTimer` _returnvalue))))

(event `StartEnemyTimer`
  (bind _blackboard (`self.Blackboard`))
  ; EnemyNotFound
  (`BlackboardComponent.SetValueAsBool` _blackboard (`self.HasLineOfSight`) false)
  (`BlackboardComponent.SetValueAsObject` _blackboard (`self.EnemyActor`) null))

(fn `UserConstructionScript`)