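; Enemy robot AI character that detects the player and can be destroyed by damage.
; AI Perception updates feed LightHandleSense, which sets CanSeePlayer from the stimulus for the player character and clears it for any other actor.
; AnyDamage subtracts from EnemyHP and destroys the actor once it reaches zero or below.
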(event `self.AIPerception.OnTargetPerceptionUpdated`
  (params (Actor :type "Actor Object Reference") (Stimulus :type "AIStimulus Structure"))
  ; Check for Player Visibility
  (`self.LightHandleSense` Actor Stimulus))

(event `self.ReceiveAnyDamage`
  (params (Damage :type "Float (single-precision)") (DamageType :type "DamageType Object Reference") (InstigatedBy :type "Controller Object Reference") (DamageCauser :type "Actor Object Reference"))
  ; Letting The Enemy Be Destroyed Upon Being Shot
  (bind _output_get (set `self.EnemyHP` (- (`self.EnemyHP`) Damage)))
  (if (<= _output_get 0.0)
    (`self.K2_DestroyActor`)))

(fn `LightHandleSense`
  (params (Actor :type "Actor Object Reference") (Stimulus :type "AIStimulus Structure"))
  (if (== Actor (`GameplayStatics.GetPlayerCharacter` 0))
    (set `self.CanSeePlayer` (`.bSuccessfullySensed` (break `AIStimulus` Stimulus)))
    (else
      (set `self.CanSeePlayer` false)))
  (return))

(fn `UserConstructionScript`)