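; BP_MissileEnemy is a shootable enemy homing missile that damages the player character and expires after a timer.
; ProjectileMovement homes on a supplied target component, while Tick separately rotates the actor to face the player.
; CollisionBox overlaps destroy it, applying damage only to BP_ThirdPersonCharacter, while blocking hits fire a radial impulse with explosion effects and sound before destruction.
; Incoming damage depletes MissileHealth and destroys it at zero.
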(event `self.ReceiveBeginPlay`
  (`GameplayStatics.PlaySoundAtLocation` "/Game/SFX/MissilieMovement.MissilieMovement" (0.0 0.0 0.0) (struct) 1.0 1.0 0.0 null null null null)
  (set `ProjectileMovementComponent.HomingTargetComponent` (`self.Homing Target Component`) (`self.ProjectileMovement`))
  (`KismetSystemLibrary.K2_SetTimerDelegate` (delegate `Destroy`) (`self.DeathTimer`)))

(event `Destroy`
  (`self.K2_DestroyActor`))

(event `self.ReceiveTick`
  (params (DeltaSeconds :type "Float (single-precision)"))
  (`self.K2_SetActorRotation` (`KismetMathLibrary.FindLookAtRotation` (`self.K2_GetActorLocation`) (`self.K2_GetActorLocation` (`GameplayStatics.GetPlayerCharacter` 0)))))

(event `self.ReceiveAnyDamage`
  (params (Damage :type "Float (single-precision)") (DamageType :type "DamageType Object Reference") (InstigatedBy :type "Controller Object Reference") (DamageCauser :type "Actor Object Reference"))
  ; Missile Destroy on Shoot
  (bind _output_get (set `self.MissileHealth` (- (`self.MissileHealth`) Damage)))
  (if (<= _output_get 0.0)
    (`self.K2_DestroyActor`)))

(event `self.Collision Box.OnComponentBeginOverlap`
  (params (OverlappedComponent :type "PrimitiveComponent Object Reference") (OtherActor :type "Actor Object Reference") (OtherComp :type "PrimitiveComponent Object Reference") (OtherBodyIndex :type Integer) (bFromSweep :type Boolean) (SweepResult :type "HitResult Structure (by ref)"))
  ; Enemy Overlap
  (if (== (`GameplayStatics.GetObjectClass` OtherActor) "/Game/ThirdPerson/Blueprints/BP_ThirdPersonCharacter.BP_ThirdPersonCharacter_C")
    (bind _asbp_third_person_character (cast `/Game/ThirdPerson/Blueprints/BP_ThirdPersonCharacter` OtherActor))
    (`GameplayStatics.ApplyDamage` _asbp_third_person_character (`self.MissileDamage`))
    (`self.K2_DestroyActor`)
    (else
      (`self.K2_DestroyActor`))))

(event `self.Collision Box.OnComponentHit`
  (params (HitComponent :type "PrimitiveComponent Object Reference") (OtherActor :type "Actor Object Reference") (OtherComp :type "PrimitiveComponent Object Reference") (NormalImpulse :type "Vector Structure") (Hit :type "HitResult Structure (by ref)"))
  (bind (_bblockinghit _binitialoverlap _time _distance _location) (`GameplayStatics.BreakHitResult` Hit))
  (`RadialForceComponent.FireImpulse` (`self.RadialForce`))
  (`GameplayStatics.SpawnEmitterAtLocation` null _location)
  (`GameplayStatics.PlaySoundAtLocation` null _location (struct) 1.0 1.0 0.0 null null null null)
  (`GameplayStatics.PlaySound2D` "/Game/StarterContent/Audio/Explosion_Cue.Explosion_Cue" 1.0 1.0 0.0 null null)
  (`self.K2_DestroyActor`))

(fn `UserConstructionScript`)