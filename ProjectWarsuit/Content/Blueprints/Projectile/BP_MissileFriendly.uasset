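; BP_MissileFriendly is a homing missile projectile that destroys AI characters on contact.
; BeginPlay passes its homing target component to ProjectileMovement and starts a timer that destroys the missile after DeathTimer.
; Every Tick it turns to face the actor returned by GetActorOfClass for BP_AIChar, independent of the homing target.
; A CollisionBox overlap with a BP_AIChar destroys both that character and the missile.
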(event `self.ReceiveBeginPlay`
  (set `ProjectileMovementComponent.HomingTargetComponent` (`self.Homing Target Component`) (`self.ProjectileMovement`))
  (`KismetSystemLibrary.K2_SetTimerDelegate` (delegate `Destroy`) (`self.DeathTimer`)))

(event `Destroy`
  (`self.K2_DestroyActor`))

(event `self.ReceiveTick`
  (params (DeltaSeconds :type "Float (single-precision)"))
  (bind _returnvalue (`GameplayStatics.GetActorOfClass` "/Game/Blueprints/EnemyRobots/AI/BP_AIChar.BP_AIChar_C"))
  (`self.K2_SetActorRotation` (`KismetMathLibrary.FindLookAtRotation` (`self.K2_GetActorLocation`) (`self.K2_GetActorLocation` _returnvalue))))

(event `self.Collision Box.OnComponentBeginOverlap`
  (params (OverlappedComponent :type "PrimitiveComponent Object Reference") (OtherActor :type "Actor Object Reference") (OtherComp :type "PrimitiveComponent Object Reference") (OtherBodyIndex :type Integer) (bFromSweep :type Boolean) (SweepResult :type "HitResult Structure (by ref)"))
  (bind _asbp_aichar (cast `/Game/Blueprints/EnemyRobots/AI/BP_AIChar` OtherActor))
  (`self.K2_DestroyActor` _asbp_aichar)
  (`self.K2_DestroyActor`))

(fn `UserConstructionScript`)