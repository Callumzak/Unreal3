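; BP_generator is a destructible generator actor that opens a moving door when damaged.
; Its Niagara effect is switched off at BeginPlay.
; The first damage event of any amount sets a Destroyed flag, activates the effect, removes the point light and calls DoorOpen on the BP_MovingDoor found by class lookup.
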(event `self.ReceiveAnyDamage`
  (params (Damage :type "Float (single-precision)") (DamageType :type "DamageType Object Reference") (InstigatedBy :type "Controller Object Reference") (DamageCauser :type "Actor Object Reference"))
  (if (not (`self.Destroyed`))
    (set `self.Destroyed` true)
    (`ActorComponent.Activate` (`self.Niagara`) false)
    (`ActorComponent.K2_DestroyComponent` (`self.PointLight`))
    (bind _returnvalue (`GameplayStatics.GetActorOfClass` "/Game/Blueprints/MovingPlatform/BP_MovingDoor.BP_MovingDoor_C"))
    (`/Game/Blueprints/MovingPlatform/BP_MovingDoor.DoorOpen` _returnvalue)))

(event `self.ReceiveBeginPlay`
  (`ActorComponent.Deactivate` (`self.Niagara`)))

(fn `UserConstructionScript`)